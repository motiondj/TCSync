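; BP_TimecodeSyncTester is a test harness actor that runs TimecodeSync checks on BeginPlay and prints results to screen.
; RunIntergreatedTest spawns a test actor and constructs the LogicTest and NetworkTest objects used by the test events.
; UDP connection, message serialization and auto role detection run after parallel 0.2-second delays, so results print after the results banner.
; Packet loss, master/slave, frame rate and system time tests exist but are unwired.
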(event `self.ReceiveBeginPlay`
  (`KismetSystemLibrary.PrintString` "TimecodeSync Test Started")
  (`KismetSystemLibrary.PrintString` "\"=== Starting Integrated TimecodeSync Tests ===\"" true true (struct :`G` 0.66 :`B` 1.0 :`A` 1.0) 5.0)
  (`self.RunIntergreatedTest`)
  (`self.UPDConnection`)
  (`self.Message Serialization`)
  (`self.Auto Role Detection`)
  (`KismetSystemLibrary.PrintString` "\"=== TimecodeSync Test Results ===\""))

(event `UPDConnection`
  ; Network Test
  (`KismetSystemLibrary.Delay` 0.2)
  (bind _returnvalue (`TimecodeSyncNetworkTest.TestUDPConnection` (`self.NetworkTest`) 12345))
  (`KismetSystemLibrary.PrintString` (`KismetStringLibrary.Conv_BoolToString` _returnvalue)))

(event `Master Slave`
  ; Logic Test
  (`KismetSystemLibrary.Delay` 0.2)
  (bind _returnvalue (`TimecodeSyncLogicTest.TestMasterSlaveSync` (`self.LogicTest`) 5.0))
  (`KismetSystemLibrary.PrintString` (`KismetStringLibrary.Conv_BoolToString` _returnvalue)))

(event `Message Serialization`
  ; Network Test
  (`KismetSystemLibrary.Delay` 0.2)
  (bind _returnvalue (`TimecodeSyncNetworkTest.TestMessageSerialization` (`self.NetworkTest`)))
  (`KismetSystemLibrary.PrintString` (`KismetStringLibrary.Conv_BoolToString` _returnvalue)))

(event `Multiple Frame Rates`
  ; Logic Test
  (`KismetSystemLibrary.Delay` 0.2)
  (bind _returnvalue (`TimecodeSyncLogicTest.TestMultipleFrameRates` (`self.LogicTest`)))
  (`KismetSystemLibrary.PrintString` (`KismetStringLibrary.Conv_BoolToString` _returnvalue)))

(event `Packet Loss`
  ; Network Test
  (`KismetSystemLibrary.Delay` 0.2)
  (bind _returnvalue (`TimecodeSyncNetworkTest.TestPacketLoss` (`self.NetworkTest`) 20.0))
  (`KismetSystemLibrary.PrintString` (`KismetStringLibrary.Conv_BoolToString` _returnvalue)))

(event `System Time Sync`
  ; Logic Test
  (`KismetSystemLibrary.Delay` 0.2)
  (bind _returnvalue (`TimecodeSyncLogicTest.TestSystemTimeSync` (`self.LogicTest`)))
  (`KismetSystemLibrary.PrintString` (`KismetStringLibrary.Conv_BoolToString` _returnvalue)))

(event `Auto Role Detection`
  ; Logic Test
  (`KismetSystemLibrary.Delay` 0.2)
  (bind _returnvalue (`TimecodeSyncLogicTest.TestAutoRoleDetection` (`self.LogicTest`)))
  (`KismetSystemLibrary.PrintString` (`KismetStringLibrary.Conv_BoolToString` _returnvalue)))

(fn `RunIntergreatedTest`
  (bind _returnvalue (`|SpawnActorFromClass` (`self.Class`) (`self.GetTransform`) "Undefined" "MultiplyWithRoot" null null))
  (set `self.TestActor` _returnvalue)
  (bind _returnvalue_2 (`|GenericCreateObject` "/Script/TimecodeSync.TimecodeSyncLogicTest"))
  (set `self.LogicTest` _returnvalue_2)
  (bind _returnvalue_3 (`|GenericCreateObject` "/Script/TimecodeSync.TimecodeSyncNetworkTest"))
  (set `self.NetworkTest` _returnvalue_3))

(fn `UserConstructionScript`)