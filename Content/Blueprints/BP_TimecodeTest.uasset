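; Test actor that exercises a Timecode object's network setup and shows the current timecode on screen.
; On BeginPlay it joins a fixed multicast group and sets up the network, then on success waits briefly before starting timecode and logging debug info.
; Tick prints the current timecode every frame, regardless of whether setup succeeded.
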(event `self.ReceiveBeginPlay`
  (bind _timecode (`self.Timecode`))
  (`TimecodeComponent.JoinMulticastGroup` _timecode "239.0.0.1")
  (bind _returnvalue (`TimecodeComponent.SetupNetwork` _timecode))
  (if _returnvalue
    (`KismetSystemLibrary.Delay` 2.0)
    (`TimecodeComponent.StartTimecode` _timecode)
    (`TimecodeComponent.LogDebugInfo` _timecode)))

(event `self.ReceiveTick`
  (params (DeltaSeconds :type "Float (single-precision)"))
  (`KismetSystemLibrary.PrintString` (`TimecodeComponent.GetCurrentTimecode` (`self.Timecode`))))

(fn `UserConstructionScript`)